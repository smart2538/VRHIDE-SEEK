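; Trap actor that opens and plays an explosion effect when another actor overlaps it, with networked state and effects.
; Overlap sets TrapOpen, whose RepNotify runs OpenTrap (only a debug print), then calls a multicast event that attaches the explosion emitter to the cube.
; The overlap path has no authority check or once-only guard; an authority-gated DoOnce route through OnTrapTouched is left unconnected.
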(event `self.ReceiveActorBeginOverlap`
  (params (OtherActor :type "Actor Object Reference"))
  (set `self.bTrapOpen` true)
  (`self.MulticastPlayFX`))

(event `MulticastPlayFX`
  (`self.PlayFX`))

(fn `OnRep_bTrapOpen`
  (if (`self.bTrapOpen`)
    (`self.OpenTrap`)))

(fn `OnTrapTouched`
  (`self.OpenTrap`)
  (`self.PlayFX`))

(fn `OpenTrap`
  (`KismetSystemLibrary.PrintString` "Trap is opened"))

(fn `PlayFX`
  (`GameplayStatics.SpawnEmitterAttached` "/Game/StarterContent/Particles/P_Explosion.P_Explosion" (`self.Cube`))
  (`KismetSystemLibrary.PrintString` "Show FX trap"))

(fn `UserConstructionScript`)