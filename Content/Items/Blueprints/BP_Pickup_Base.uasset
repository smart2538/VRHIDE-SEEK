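; Base pickup actor that motion controllers grab and drop by toggling mesh physics and attachment, with a lifetime readout as text or scaled box.
; Call events pass through Multi events to the setters, which show the indicator, turn it partway toward the VR or third-person camera, and hide it after one second.
; Both indicators share one timer handle, and the box's Y scale divides remaining range by zero.
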(event `CallSetTextLifeTime`
  (params (LifeTime :type "Float (double-precision)"))
  ;[1 1 1] Text Life Time
  (`self.MultiTextLifeTime` LifeTime))

(event `MultiTextLifeTime`
  (params (LifeTime :type "Float (double-precision)"))
  ;[1 1 1] Text Life Time
  (`self.SetTextLifeTime` LifeTime))

(event `/Game/VirtualRealityBP/Blueprints/PickupActorInterface.Pickup`
  (params (AttachTo :type "SceneComponent Object Reference"))
  (`PrimitiveComponent.SetSimulatePhysics` (`self.StaticMeshComponent`) false)
  (`SceneComponent.K2_AttachToComponent` (`self.K2_GetRootComponent`) AttachTo "None" "KeepWorld" "KeepWorld" "KeepWorld" false))

(event `CallSetBoxLifeTime`
  (params (LifeTime :type "Float (double-precision)") (MaxLifeTime :type "Float (double-precision)"))
  ;[1 1 1] Box Life Time
  (`self.MultiBoxLifeTime` LifeTime MaxLifeTime))

(event `MultiBoxLifeTime`
  (params (LifeTime :type "Float (double-precision)") (MaxLifeTime :type "Float (double-precision)"))
  ;[1 1 1] Box Life Time
  (`self.SetBoxLifeTime` LifeTime MaxLifeTime))

(event `/Game/VirtualRealityBP/Blueprints/PickupActorInterface.Drop`
  (`PrimitiveComponent.SetSimulatePhysics` (`self.StaticMeshComponent`) true)
  (`self.K2_DetachFromActor` "KeepWorld" "KeepWorld" "KeepWorld"))

(event `/Game/VirtualRealityBP/Blueprints/PickupActorInterface.AttemptCallShowTextLifeTime`
  (params (LifeTime :type "Float (single-precision)") (MaxLifeTime :type "Float (single-precision)"))
  (`self.SetBoxLifeTime` LifeTime MaxLifeTime))

(fn `ActiveBoxLifeTime`
  (`SceneComponent.SetVisibility` (`self.BoxLifeTime`) true false))

(fn `ActiveTextLifeTime`
  (`SceneComponent.SetVisibility` (`self.TextLifeTime`) true false))

(fn `DeactiveBoxLifeTime`
  (`SceneComponent.SetVisibility` (`self.BoxLifeTime`) false false))

(fn `DeactiveTextLifeTime`
  (`SceneComponent.SetVisibility` (`self.TextLifeTime`) false false))

(fn `RotateBoxLifeTime`
  (bind _returnvalue (`GameplayStatics.GetPlayerPawn` 0))
  (bind _boxlifetime (`self.BoxLifeTime`))
  (if (== (`GameplayStatics.GetObjectClass` _returnvalue) "/Game/VirtualRealityBP/Blueprints/MotionControllerPawn.MotionControllerPawn_C")
    (bind _asmotion_controller_pawn (cast `/Game/VirtualRealityBP/Blueprints/MotionControllerPawn` _returnvalue))
    (`SceneComponent.K2_SetWorldRotation` _boxlifetime (`KismetMathLibrary.RLerp` (`SceneComponent.K2_GetComponentRotation` _boxlifetime) (`KismetMathLibrary.MakeRotator` (.roll (`SceneComponent.K2_GetComponentRotation` (`/Game/VirtualRealityBP/Blueprints/MotionControllerPawn.Camera` _asmotion_controller_pawn))) (* (.pitch (`SceneComponent.K2_GetComponentRotation` (`/Game/VirtualRealityBP/Blueprints/MotionControllerPawn.Camera` _asmotion_controller_pawn))) -1.0) (+ (.yaw (`SceneComponent.K2_GetComponentRotation` (`/Game/VirtualRealityBP/Blueprints/MotionControllerPawn.Camera` _asmotion_controller_pawn))) 180.0)) 0.5 true) false false)
    (else
      (bind _asthird_person_pickup (cast `/Game/ThirdPersonBP/Blueprints/ThirdPersonPickup` _returnvalue))
      (`SceneComponent.K2_SetWorldRotation` _boxlifetime (`KismetMathLibrary.RLerp` (`SceneComponent.K2_GetComponentRotation` _boxlifetime) (`KismetMathLibrary.MakeRotator` (.roll (`SceneComponent.K2_GetComponentRotation` (`/Game/ThirdPersonBP/Blueprints/ThirdPersonPickup.FollowCamera` _asthird_person_pickup))) (* (.pitch (`SceneComponent.K2_GetComponentRotation` (`/Game/ThirdPersonBP/Blueprints/ThirdPersonPickup.FollowCamera` _asthird_person_pickup))) -1.0) (+ (.yaw (`SceneComponent.K2_GetComponentRotation` (`/Game/ThirdPersonBP/Blueprints/ThirdPersonPickup.FollowCamera` _asthird_person_pickup))) 180.0)) 0.5 true) false false))))

(fn `RotateTextLifeTime`
  (bind _returnvalue (`GameplayStatics.GetPlayerPawn` 0))
  (if (== (`GameplayStatics.GetObjectClass` _returnvalue) "/Game/VirtualRealityBP/Blueprints/BP_MotionController.BP_MotionController_C")
    (bind _asmotion_controller_pawn (cast `/Game/VirtualRealityBP/Blueprints/MotionControllerPawn` _returnvalue))
    (`SceneComponent.K2_SetWorldRotation` (`self.TextLifeTime`) (`KismetMathLibrary.RLerp` (`SceneComponent.K2_GetComponentRotation` (`self.TextLifeTime`)) (`KismetMathLibrary.MakeRotator` (.roll (`SceneComponent.K2_GetComponentRotation` (`/Game/VirtualRealityBP/Blueprints/MotionControllerPawn.Camera` _asmotion_controller_pawn))) (* (.pitch (`SceneComponent.K2_GetComponentRotation` (`/Game/VirtualRealityBP/Blueprints/MotionControllerPawn.Camera` _asmotion_controller_pawn))) -1.0) (+ (.yaw (`SceneComponent.K2_GetComponentRotation` (`/Game/VirtualRealityBP/Blueprints/MotionControllerPawn.Camera` _asmotion_controller_pawn))) 180.0)) 0.5 true) false false)
    (else
      (bind _asthird_person_pickup (cast `/Game/ThirdPersonBP/Blueprints/ThirdPersonPickup` _returnvalue))
      (`SceneComponent.K2_SetWorldRotation` (`self.TextLifeTime`) (`KismetMathLibrary.RLerp` (`SceneComponent.K2_GetComponentRotation` (`self.TextLifeTime`)) (`KismetMathLibrary.MakeRotator` (.roll (`SceneComponent.K2_GetComponentRotation` (`/Game/ThirdPersonBP/Blueprints/ThirdPersonPickup.FollowCamera` _asthird_person_pickup))) (* (.pitch (`SceneComponent.K2_GetComponentRotation` (`/Game/ThirdPersonBP/Blueprints/ThirdPersonPickup.FollowCamera` _asthird_person_pickup))) -1.0) (+ (.yaw (`SceneComponent.K2_GetComponentRotation` (`/Game/ThirdPersonBP/Blueprints/ThirdPersonPickup.FollowCamera` _asthird_person_pickup))) 180.0)) 0.5 true) false false))))

(fn `SetBoxLifeTime`
  (params (LifeTime :type "Float (double-precision)") (MaxLifeTime :type "Float (double-precision)"))
  (bind _boxlifetime (`self.BoxLifeTime`))
  (`KismetSystemLibrary.K2_ClearAndInvalidateTimerHandle` (`self.LifeTimeHandle`))
  (`SceneComponent.SetRelativeScale3D` _boxlifetime (`KismetMathLibrary.MakeVector` (.x (`SceneComponent.RelativeScale3D` _boxlifetime)) (/ (- MaxLifeTime LifeTime) 0.0) (.z (`SceneComponent.RelativeScale3D` _boxlifetime))))
  (`self.ActiveBoxLifeTime`)
  (`self.RotateBoxLifeTime`)
  (bind _returnvalue (`KismetSystemLibrary.K2_SetTimer` null "DeactiveBoxLifeTime" 1.0))
  (set `self.LifeTimeHandle` _returnvalue))

(fn `SetTextLifeTime`
  (params (LifeTime :type "Float (double-precision)"))
  (`KismetSystemLibrary.K2_ClearAndInvalidateTimerHandle` (`self.LifeTimeHandle`))
  (`self.ActiveTextLifeTime`)
  (`self.RotateTextLifeTime`)
  (`TextRenderComponent.K2_SetText` (`self.TextLifeTime`) (`KismetTextLibrary.Conv_DoubleToText` LifeTime "HalfToEven"))
  (bind _returnvalue (`KismetSystemLibrary.K2_SetTimer` null "DeactiveTextLifeTime" 1.0))
  (set `self.LifeTimeHandle` _returnvalue))

(fn `UserConstructionScript`)