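; Player state for a hide-and-seek game, tracking a player's role, status and carried collectible count.
; Collectible events and helper functions raise, lower, reset and query the count, keeping increments and decrements between zero and a limit.
; Winning asks HideSeekGameState to load the win scene, then marks the player escaped and calls the game state's PlayerLoseHealth.
; Preparing to die drops a collectible and changes status.
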(event `self.ReceiveTick`
  (params (DeltaSeconds :type "Float (single-precision)")))

(event `ResetCollectible`
  (set `self.NumberOfCollectibles` 0))

(event `recieveCollectibleObject`
  (`self.IncrementCollectible`))

(event `dropCollectible`
  (`self.DecrementCollectible`))

(event `CallWinGame`
  (bind _ashide_seek_game_state (cast `/Game/ThirdPersonBP/Blueprints/HideSeekGameState` (`GameplayStatics.GetGameState`)))
  (`/Game/ThirdPersonBP/Blueprints/HideSeekGameState.LoadPlayerWinScene` _ashide_seek_game_state null)
  (`self.OnPlayerEscaped`))

(event `PrepareToDie`
  (`self.dropCollectible`)
  (set `self.Status` "NewEnumerator2"))

(event `OnPlayerEscaped`
  (set `self.Status` "NewEnumerator1")
  (bind _ashide_seek_game_state (cast `/Game/ThirdPersonBP/Blueprints/HideSeekGameState` (`GameplayStatics.GetGameState`)))
  (`/Game/ThirdPersonBP/Blueprints/HideSeekGameState.playerLoseHealth` _ashide_seek_game_state))

(fn `CountCollectibleObjects`
  (returns (CollectibleCount :type Integer))
  (return (`self.NumberOfCollectibles`)))

(fn `DecrementCollectible`
  (if (>= (- (`self.NumberOfCollectibles`) 1) 0)
    (set `self.NumberOfCollectibles` (- (`self.NumberOfCollectibles`) 1))))

(fn `GetPlayerRole`
  (returns (Role :type "/Game/Blueprints/PlayerRoleEnum Enum"))
  (return (`self.PlayerRole`)))

(fn `IncrementCollectible`
  (if (<= (+ (`self.NumberOfCollectibles`) 1) (`self.CollectibleLimit`))
    (set `self.NumberOfCollectibles` (+ (`self.NumberOfCollectibles`) 1))))

(fn `isPlayerHaveCollectibleObject`
  (returns (isPlayerHaveCollectibleObject :type Boolean))
  (return (> (`self.NumberOfCollectibles`) 0)))

(fn `ResetCollectibleCounts`
  (set `self.NumberOfCollectibles` 0))

(fn `UserConstructionScript`)