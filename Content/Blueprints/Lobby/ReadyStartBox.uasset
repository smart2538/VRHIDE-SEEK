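; VR lobby box that players pick up and drop, serving as a physical ready/start trigger.
; Tick polls LobbyGM's CanWeStart, then once swaps the box material, reveals its text labels and activates its particle system.
; Pickup and Drop toggle physics and attachment to the motion controller.
; Destroying it on the server, when the first player controls a MotionControllerPawn, calls OnActivatedReadyStart on that player's lobby menu widget.
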(event `/Game/VirtualRealityBP/Blueprints/PickupActorInterface.Pickup`
  (params (AttachTo :type "SceneComponent Object Reference"))
  (`PrimitiveComponent.SetSimulatePhysics` (`self.StaticMeshComponent`) false)
  (`SceneComponent.K2_AttachToComponent` (`self.K2_GetRootComponent`) AttachTo "None" "KeepWorld" "KeepWorld" "KeepWorld" false))

(event `self.ReceiveDestroyed`
  (bind _returnvalue (`GameplayStatics.GetPlayerController` 0))
  (if (and (`KismetSystemLibrary.IsServer`) (== (`GameplayStatics.GetObjectClass` (`Controller.K2_GetPawn` _returnvalue)) "/Game/VirtualRealityBP/Blueprints/MotionControllerPawn.MotionControllerPawn_C"))
    (bind _aslobby_pc (cast `/Game/Blueprints/Lobby/LobbyPC` _returnvalue))
    (`/Game/UI/Lobby/LobbyMenu.OnActivatedReadyStart` (`/Game/Blueprints/Lobby/LobbyPC.LobbyMenuWB` _aslobby_pc))))

(event `self.ReceiveTick`
  (params (DeltaSeconds :type "Float (single-precision)"))
  (if (`/Game/Blueprints/Lobby/LobbyGM.CanWeStart?` (cast `/Game/Blueprints/Lobby/LobbyGM` (`GameplayStatics.GetGameMode`) :!pure true))
    (`/Engine/EditorBlueprintResources/StandardMacros.DoOnce` false
      (:`Completed`
        (`PrimitiveComponent.SetMaterial` (`self.StaticMeshComponent`) 0 "/Game/MixamoAnimPack/Mixamo_Alpha/Materials/Alpha_Body.Alpha_Body")
        (`SceneComponent.SetVisibility` (`self.TextRender2`) true false)
        (`SceneComponent.SetVisibility` (`self.TextRender1`) true false)
        (`SceneComponent.SetVisibility` (`self.TextRender3`) true false)
        (`SceneComponent.SetVisibility` (`self.TextRender4`) true false)
        (`SceneComponent.SetVisibility` (`self.TextRender5`) true false)
        (`SceneComponent.SetVisibility` (`self.TextRender6`) true false)
        (`SceneComponent.SetVisibility` (`self.TextRender7`) true false)
        (`SceneComponent.SetVisibility` (`self.TextRender`) true false)
        (`ActorComponent.SetActive` (`self.ParticleSystem`) true true)))))

(event `/Game/VirtualRealityBP/Blueprints/PickupActorInterface.Drop`
  (`PrimitiveComponent.SetSimulatePhysics` (`self.StaticMeshComponent`) true)
  (`self.K2_DetachFromActor` "KeepWorld" "KeepWorld" "KeepWorld"))

(fn `UserConstructionScript`)